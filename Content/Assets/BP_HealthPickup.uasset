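; BP_HealthPickup is a pickup that adds a Kimchi icon to the HUD health bar when BP_Character overlaps it.
; It reaches the health bar's horizontal box through player 0's BP_MyOwnHUD and constructs a new Image there only while fewer than five children exist.
; The box's child count is the only health state touched, and the pickup destroys itself only when an icon is added.
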(event EventBeginPlay)

(event Collision|EventActorBeginOverlap
  (params (OtherActor :type Actor%20Object%20Reference))
  (Utilities|Casting|CastToBP_Character OtherActor)
  (bind _asbp_my_own_hud (Utilities|Casting|CastToBP_MyOwnHUD (HUD|GetHUD (Game|GetPlayerController 0))))
  (if (< (Utilities|Array|Length (Class|PanelWidget|GetAllChildren (Variables|/Game/Assets/WBP_HealthBar.WBP_HealthBar_C|GetHorizontalBox_40 (Variables|/Game/Character/BP_MyOwnHUD.BP_MyOwnHUD_C|GetWBP_HealthBar _asbp_my_own_hud)))) 5)
    (bind _returnvalue (Game|ConstructObjectfromClass "/Script/UMG.Image" "/Game/Assets/Kimchi.Kimchi"))
    (Appearance|SetBrushfromTexture _returnvalue "/Game/Assets/Kimchi.Kimchi" true)
    (Class|HorizontalBox|AddChildtoHorizontalBox (Variables|/Game/Assets/WBP_HealthBar.WBP_HealthBar_C|GetHorizontalBox_40 (Variables|/Game/Character/BP_MyOwnHUD.BP_MyOwnHUD_C|GetWBP_HealthBar _asbp_my_own_hud)) _returnvalue)
    (Actor|DestroyActor)))

(event EventTick
  (params (DeltaSeconds :type Float%20%28single-precision%29)))

(fn ConstructionScript)