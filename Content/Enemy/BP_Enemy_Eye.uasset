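; BP_Enemy_Eye is a Paper2D eye enemy that patrols, attacks the player in melee and dies from damage.
; It walks slowly forward and turns 180 degrees when EdgeDetection ends an overlap.
; PlayerDetection switches it between run and attack flipbooks, with attack frame 6 calling Hit once on a player inside the HitBox.
; Damage briefly adds a blood flipbook and reduces Health, ending in a death animation and delayed destruction.
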(event OnComponentEndOverlap(EdgeDetection)
  (params (OverlappedComponent :type Primitive%20Component%20Object%20Reference) (OtherActor :type Actor%20Object%20Reference) (OtherComp :type Primitive%20Component%20Object%20Reference) (OtherBodyIndex :type Integer))
  (Transformation|SetActorRotation (Math|Rotator|CombineRotators (Transformation|GetActorRotation) "0,180.000000, 0")))

(event OnComponentBeginOverlap(PlayerDetection)
  (params (OverlappedComponent :type Primitive%20Component%20Object%20Reference) (OtherActor :type Actor%20Object%20Reference) (OtherComp :type Primitive%20Component%20Object%20Reference) (OtherBodyIndex :type Integer) (bFromSweep :type Boolean) (SweepResult :type Hit%20Result%20Structure%20%28by%20ref%29))
  (bind _asbp_character (Utilities|Casting|CastToBP_Character OtherActor))
  (Sprite|SetFlipbook (Variables|Default|GetSprite) "/Game/Enemy/FB_Attack_eye.FB_Attack_eye")
  (Transformation|SetActorRotation (Math|Rotator|MakeRotator 0.0 0.0 (.yaw (Math|Rotator|FindLookatRotation (Transformation|GetActorLocation) (Transformation|GetActorLocation _asbp_character)))))
  (Variables|Default|SetbIsAttacking true))

(event OnComponentEndOverlap(PlayerDetection)
  (params (OverlappedComponent :type Primitive%20Component%20Object%20Reference) (OtherActor :type Actor%20Object%20Reference) (OtherComp :type Primitive%20Component%20Object%20Reference) (OtherBodyIndex :type Integer))
  (Utilities|Casting|CastToBP_Character OtherActor)
  (Sprite|SetFlipbook (Variables|Default|GetSprite) "/Game/Enemy/FB_RunEye.FB_RunEye")
  (Variables|Default|SetbIsAttacking false))

(event Custom|BloodSpawn
  (bind _returnvalue (AddComponent|AddPaperFlipbookComponent false))
  (Utilities|FlowControl|Delay 0.2)
  (Components|DestroyComponent _returnvalue))

(event EventTick
  (params (DeltaSeconds :type Float%20%28single-precision%29))
  (if (not (Variables|Default|GetbIsDeath))
    (if (Variables|Default|GetbIsAttacking)
      (if (== (Class|PaperFlipbookComponent|GetPlaybackPositioninFrames (Variables|Default|GetSprite)) 6)
        (if (Collision|IsOverlappingActor (Variables|Default|GetHitBox) (Variables|Default|GetBP_Character) :!class /Script/Engine.PrimitiveComponent)
          (Utilities|FlowControl|DoOnce false :!label _label
            (:Completed
              (Default|Hit (Variables|Default|GetBP_Character)))))
        (else
          (goto _label Reset)))
      (else
        (Pawn|Input|AddMovementInput (Transformation|GetActorForwardVector) 0.1 false)))))

(event Game|Damage|EventAnyDamage
  (params (Damage :type Float%20%28single-precision%29) (DamageType :type Damage%20Type%20Object%20Reference) (InstigatedBy :type Controller%20Object%20Reference) (DamageCauser :type Actor%20Object%20Reference))
  (CallFunction|BloodSpawn)
  (bind _output_get (Variables|Default|SetHealth (- (Variables|Default|GetHealth) Damage)))
  (if (<= _output_get 0.0)
    (Sprite|SetFlipbook (Variables|Default|GetSprite) "/Game/Enemy/FB_DeathEye.FB_DeathEye")
    (Components|Activation|Deactivate (Variables|Character|GetCharacterMovement))
    (Variables|Default|SetbIsDeath true)
    (Components|Timeline|SetLooping (Variables|Default|GetSprite) true)
    (Utilities|FlowControl|Delay 1.0)
    (Actor|DestroyActor)))

(event EventBeginPlay
  (bind _asbp_character (Utilities|Casting|CastToBP_Character (Game|GetPlayerCharacter 0)))
  (Variables|Default|SetBP_Character _asbp_character))

(fn ConstructionScript)