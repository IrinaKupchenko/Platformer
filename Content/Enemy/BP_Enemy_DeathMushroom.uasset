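; Paper2D mushroom enemy that walks forward, turns around when its edge detector stops overlapping, and attacks the player.
; Player detection switches run and attack flipbooks and faces the player; on a specific attack frame, a hitbox overlap triggers one hit on the character.
; Damage spawns brief blood effects and reduces health; death plays its flipbook, fires the enemy-death call, destroys the actor and may drop a health pickup.
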(event OnComponentEndOverlap(EdgeDetection)
  (params (OverlappedComponent :type Primitive%20Component%20Object%20Reference) (OtherActor :type Actor%20Object%20Reference) (OtherComp :type Primitive%20Component%20Object%20Reference) (OtherBodyIndex :type Integer))
  (Transformation|SetActorRotation (Math|Rotator|CombineRotators (Transformation|GetActorRotation) "0,180.000000, 0")))

(event OnComponentBeginOverlap(PlayerDetection)
  (params (OverlappedComponent :type Primitive%20Component%20Object%20Reference) (OtherActor :type Actor%20Object%20Reference) (OtherComp :type Primitive%20Component%20Object%20Reference) (OtherBodyIndex :type Integer) (bFromSweep :type Boolean) (SweepResult :type Hit%20Result%20Structure%20%28by%20ref%29))
  (bind _asbp_character (Utilities|Casting|CastToBP_Character OtherActor))
  (Sprite|SetFlipbook (Variables|Default|GetSprite) "/Game/Enemy/FB_AttackMush.FB_AttackMush")
  (Transformation|SetActorRotation (Math|Rotator|MakeRotator 0.0 0.0 (.yaw (Math|Rotator|FindLookatRotation (Transformation|GetActorLocation) (Transformation|GetActorLocation _asbp_character)))))
  (Variables|Default|SetbIsAttacking true))

(event OnComponentEndOverlap(PlayerDetection)
  (params (OverlappedComponent :type Primitive%20Component%20Object%20Reference) (OtherActor :type Actor%20Object%20Reference) (OtherComp :type Primitive%20Component%20Object%20Reference) (OtherBodyIndex :type Integer))
  (Utilities|Casting|CastToBP_Character OtherActor)
  (Sprite|SetFlipbook (Variables|Default|GetSprite) "/Game/Enemy/FB_RunMush.FB_RunMush")
  (Variables|Default|SetbIsAttacking false))

(event Custom|BloodSpawn
  (bind _returnvalue (AddComponent|AddPaperFlipbookComponent false))
  (Utilities|FlowControl|Delay 0.2)
  (Components|DestroyComponent _returnvalue))

(event EventTick
  (params (DeltaSeconds :type Float%20%28single-precision%29))
  (bind _bp_character (Variables|Default|GetBP_Character))
  (if (not (Variables|Default|GetbIsDeath))
    (if (Variables|Default|GetbIsAttacking)
      (if (== (Class|PaperFlipbookComponent|GetPlaybackPositioninFrames (Variables|Default|GetSprite)) 6)
        (if (Collision|IsOverlappingActor (Variables|Default|GetHitBox) (Variables|Default|GetBP_Character) :!class /Script/Engine.PrimitiveComponent)
          (Utilities|FlowControl|DoOnce false :!label _label
            (:Completed
              (Default|Hit _bp_character)
              (Audio|PlaySoundatLocation "/Game/Assets/Sounds/HitThePlayer.HitThePlayer" (Transformation|GetActorLocation _bp_character) "0, 0, 0" 1.0 1.0 0.0 0 0 0))))
        (else
          (goto _label Reset)))
      (else
        (Pawn|Input|AddMovementInput (Transformation|GetActorForwardVector) 0.1 false)))))

(event Game|Damage|EventAnyDamage
  (params (Damage :type Float%20%28single-precision%29) (DamageType :type Damage%20Type%20Object%20Reference) (InstigatedBy :type Controller%20Object%20Reference) (DamageCauser :type Actor%20Object%20Reference))
  (Audio|PlaySoundatLocation "/Game/Assets/Sounds/HitTheEnemy_Cue.HitTheEnemy_Cue" (Transformation|GetActorLocation) "0, 0, 0" 1.0 1.0 0.0 0 0 0)
  (CallFunction|BloodSpawn)
  (bind _output_get (Variables|Default|SetHealth (- (Variables|Default|GetHealth) Damage)))
  (if (<= _output_get 0.0)
    (Sprite|SetFlipbook (Variables|Default|GetSprite) "/Game/Enemy/FB_DeathMush.FB_DeathMush")
    (Components|Activation|Deactivate (Variables|Character|GetCharacterMovement))
    (Variables|Default|SetbIsDeath true)
    (Components|Timeline|SetLooping (Variables|Default|GetSprite) true)
    (Utilities|FlowControl|Delay 1.0)
    (Default|CallOnEnemyDeath)
    (Actor|DestroyActor)
    (if (< (Math|Random|RandomFloatinRange 0.0 1.0) 0.3)
      (Game|SpawnActorfromClass "/Game/Assets/BP_HealthPickup.BP_HealthPickup_C" (Math|Conversions|ToTransform(Vector) (Transformation|GetActorLocation)) "Undefined" 0 0))))

(event EventBeginPlay
  (bind _asbp_character (Utilities|Casting|CastToBP_Character (Game|GetPlayerCharacter 0)))
  (Variables|Default|SetBP_Character _asbp_character))

(fn ConstructionScript)