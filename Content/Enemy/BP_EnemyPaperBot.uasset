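; BP_EnemyPaperBot is an enemy that moves slowly along its forward axis in response to the player's position.
; Each Tick casts the player pawn to BP_Character and compares X positions to pick the sign of the movement input.
; Both branches then set an equivalent half-turn yaw (±180), so facing never differs and, once rotated, the input points away from the player along X.
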(event EventBeginPlay)

(event Collision|EventActorBeginOverlap
  (params (OtherActor :type Actor%20Object%20Reference)))

(event EventTick
  (params (DeltaSeconds :type Float%20%28single-precision%29))
  (bind _returnvalue (Transformation|GetActorForwardVector))
  (bind _asbp_character (Utilities|Casting|CastToBP_Character (Game|GetPlayerCharacter 0)))
  (if (> (.x (Transformation|GetActorLocation _asbp_character)) (.x (Transformation|GetActorLocation)))
    (Pawn|Input|AddMovementInput _returnvalue 0.1 false)
    (Transformation|SetActorRotation (Math|Rotator|MakeRotator 0.0 0.0 -1.8e+02))
    (else
      (Pawn|Input|AddMovementInput _returnvalue -0.1 false)
      (Transformation|SetActorRotation (Math|Rotator|MakeRotator 0.0 0.0 1.8e+02)))))

(fn ConstructionScript)