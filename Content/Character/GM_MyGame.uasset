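; Game mode that runs a kill-all-enemies level and opens L_MainLevel_2 when the last enemy dies.
; BeginPlay sets game-only input without a cursor, starts the music, then gathers Death Mushroom and Eye enemies.
; Both searches feed one shared chain that totals RemainingEnemiesCount and binds each enemy's death event to OnEnemyDied.
; OnEnemyDied decrements and prints the count, triggering the level change at zero.
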(event Custom|OnEnemyDied
  (bind _result (Math|Integer|DecrementInt (Variables|Default|GetRemainingEnemiesCount))
    (:%20%20
      (Development|PrintString (Utilities|String|ToString(Integer) _result))
      (if (== _result 0)
        (Game|OpenLevel(byName) "L_MainLevel_2")))))

(event EventBeginPlay
  (bind _returnvalue (Game|GetPlayerController 0))
  (Variables|/Script/Engine.PlayerController|SetbShowMouseCursor _returnvalue false)
  (Input|SetInputModeGameOnly _returnvalue)
  (Audio|PlaySound2D "/Game/MainMenuSystem/Widgets/Assets/Sounds/Electric_Pulse_Paradise.Electric_Pulse_Paradise" 0.3 1.0 0.0 0 0)
  (Utilities|FlowControl|Sequence
    (:then_0
      (bind _outactors (Actor|GetAllActorsOfClass "/Game/Enemy/BP_Enemy_DeathMushroom.BP_Enemy_DeathMushroom_C")))
    (:then_1
      (bind _outactors_2 (Actor|GetAllActorsOfClass "/Game/Enemy/BP_Enemy_Eye.BP_Enemy_Eye_C"))))
  (Variables|Default|SetRemainingEnemiesCount (+ (Utilities|Array|Length _outactors) (Utilities|Array|Length _outactors_2)))
  (Utilities|FlowControl|Sequence
    (:then_0
      (for _array_element _outactors
        (EventDispatchers|BindEventtoOnEnemyDeath _array_element (delegate Custom|OnEnemyDied))))
    (:then_1
      (for _array_element_2 _outactors_2
        (EventDispatchers|BindEventtoOnEnemyDeath _array_element_2 (delegate Custom|OnEnemyDied))))))

(event EventTick
  (params (DeltaSeconds :type Float%20%28single-precision%29)))

(fn ConstructionScript)