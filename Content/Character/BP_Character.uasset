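; Player character for a 2D Paper2D side-view game, with movement, jump, dash, two-step sword attack and obelisk-triggered level loading.
; Enhanced Input and movement events swap and rotate the flipbook sprite, with IsJumping gating run animation and re-jumps.
; Standing attacks damage PaperCharacters overlapping the HitBox.
; Trap overlaps remove a HUD health-bar child, and losing the last plays death, disables input and starts a timer.
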(event OnFinishedPlaying(Sprite)
  (Sprite|SetFlipbook (Variables|Default|GetSprite) "/Game/Character/FlipBooks_Cyber/FB_Idle.FB_Idle")
  (Components|Timeline|SetLooping (Variables|Default|GetSprite) true)
  (if (not (Audio|Components|Audio|IsPlaying (Variables|Default|GetSprite)))
    (Audio|Components|Audio|Play (Variables|Default|GetSprite))))

(event OnComponentBeginOverlap(CapsuleComponent)
  (params (OverlappedComponent :type Primitive%20Component%20Object%20Reference) (OtherActor :type Actor%20Object%20Reference) (OtherComp :type Primitive%20Component%20Object%20Reference) (OtherBodyIndex :type Integer) (bFromSweep :type Boolean) (SweepResult :type Hit%20Result%20Structure%20%28by%20ref%29))
  (Utilities|Casting|CastToBP_Trap OtherActor)
  (Audio|PlaySoundatLocation "/Game/Assets/Sounds/HitTheEnemy_Cue.HitTheEnemy_Cue" (Transformation|GetActorLocation) "0, 0, 0" 0.3 1.0 0.0 0 0 0)
  (CallFunction|Hit))

(event Input|EnhancedActionEvents|EnhancedInputActionIA_MoveForward
  (params (ActionValue :type Float%20%28single-precision%29) (ElapsedSeconds :type Float%20%28single-precision%29) (TriggeredSeconds :type Float%20%28single-precision%29))
  (bind _sprite (Variables|Default|GetSprite))
  (:Canceled
    (Sprite|SetFlipbook (Variables|Default|GetSprite) "/Game/Character/FlipBooks_Cyber/FB_Idle.FB_Idle" :!label _label))
  (:Triggered
    (Pawn|Input|AddMovementInput (Transformation|GetActorForwardVector) ActionValue false)
    (if (not (Variables|Default|GetbIsJumping))
      (Sprite|SetFlipbook (Variables|Default|GetSprite) "/Game/Character/FlipBooks_Cyber/FB_Run.FB_Run")
      (if (> ActionValue 0.0)
        (Transformation|SetWorldRotation _sprite "0, 0, 0" false false)
        (else
          (Transformation|SetWorldRotation _sprite "0,-180.000000, 0" false false)))))
  (:Completed
    (goto _label)))

(event Input|EnhancedActionEvents|EnhancedInputActionIA_Jump
  (params (ActionValue :type Boolean) (ElapsedSeconds :type Float%20%28single-precision%29) (TriggeredSeconds :type Float%20%28single-precision%29))
  (Utilities|FlowControl|DoOnce false
    (:Completed
      (Audio|SpawnSoundatLocation "/Game/MainMenuSystem/Widgets/Assets/Sounds/Jump.Jump" (Transformation|GetActorLocation) "0, 0, 0" 0.4 1.0 0.1 0 0)
      (Variables|Default|SetbIsJumping true)
      (Character|Jump)
      (Sprite|SetFlipbook (Variables|Default|GetSprite) "/Game/Character/FlipBooks_Cyber/FB_Jump.FB_Jump"))))

(event Input|EnhancedActionEvents|EnhancedInputActionIA_Attack
  (params (ActionValue :type Boolean) (ElapsedSeconds :type Float%20%28single-precision%29) (TriggeredSeconds :type Float%20%28single-precision%29))
  (if (== (Math|Vector|VectorLength (Transformation|GetVelocity)) 0.0)
    (CallFunction|Attack)
    (Audio|PlaySound2D "/Game/Assets/Sounds/SwordSwing_Cue.SwordSwing_Cue" 1.0 (Math|Random|RandomFloatinRange 1.0 1.3) 0.0 0 0)
    (switch int (Variables|Default|GetAttackIndex)
      (:0
        (Sprite|SetFlipbook (Variables|Default|GetSprite) (Utilities|Array|Get(acopy) (Variables|Default|GetAttacksArray) (Variables|Default|GetAttackIndex)))
        (bind _result (Math|Integer|IncrementInt (Variables|Default|GetAttackIndex))
          (:%20%20
            (Variables|Default|SetAttackIndex _result)
            (Components|Timeline|SetLooping (Variables|Default|GetSprite) false))))
      (:1
        (Sprite|SetFlipbook (Variables|Default|GetSprite) (Utilities|Array|Get(acopy) (Variables|Default|GetAttacksArray) (Variables|Default|GetAttackIndex)))
        (Components|Timeline|SetLooping (Variables|Default|GetSprite) false)
        (Variables|Default|SetAttackIndex 0)))))

(event Input|EnhancedActionEvents|EnhancedInputActionIA_Interact
  (params (ActionValue :type Float%20%28single-precision%29) (ElapsedSeconds :type Float%20%28single-precision%29) (TriggeredSeconds :type Float%20%28single-precision%29))
  (bind _currentinteractableobelisk (Variables|Default|GetCurrentInteractableObelisk))
  (if (Variables|/Game/Assets/BP_Obelisk.BP_Obelisk_C|GetCurrentInteractableObelisk%20 _currentinteractableobelisk)
    (Utilities|IsValid _currentinteractableobelisk
      (:Is%20Valid
        (Game|OpenLevel(byName) "L_MainLevel")))))

(event EventBeginPlay
  (Utilities|FlowControl|Sequence
    (:then_0
      (bind _asbp_my_own_hud (Utilities|Casting|CastToBP_MyOwnHUD (HUD|GetHUD (Game|GetPlayerController 0))))
      (Variables|Default|SetAs%20BP%20My%20Own%20HUD _asbp_my_own_hud))
    (:then_1
      (bind _asmy_controler (Utilities|Casting|CastToMyControler (Pawn|GetController)))
      (Input|AddMappingContext (PlayerController|LocalPlayerSubsystems|GetEnhancedInputLocalPlayerSubsystem _asmy_controler) "/Game/Character/IMC_Movement.IMC_Movement" 0))))

(event EventOnLanded
  (params (Hit :type Hit%20Result%20Structure%20%28by%20ref%29))
  (Audio|SpawnSoundatLocation "/Game/MainMenuSystem/Widgets/Assets/Sounds/Land.Land" (Transformation|GetActorLocation) "0, 0, 0" 0.5 1.0 0.0 0 0)
  (Variables|Default|SetbIsJumping false)
  (Components|Timeline|SetLooping (Variables|Default|GetSprite) true)
  (Sprite|SetFlipbook (Variables|Default|GetSprite) "/Game/Character/FlipBooks_Cyber/FB_Idle.FB_Idle"))

(event EventTick
  (params (DeltaSeconds :type Float%20%28single-precision%29))
  (Utilities|FlowControl|Sequence
    (:then_0
      (if (not (Variables|Default|GetbIsJumping))
        (Utilities|FlowControl|DoOnce false) ; enters at Reset
      ))
    (:then_1
      (if (< (.z (Transformation|GetVelocity)) 0.0)
        (Sprite|SetFlipbook (Variables|Default|GetSprite) "/Game/Character/FlipBooks_Cyber/FB_Jump.FB_Jump")))))

(event Input|KeyboardEvents|LeftShift
  (params (Key :type Key%20Structure :default "None"))
  (:Pressed
    (Audio|SpawnSoundatLocation "/Game/Assets/Sounds/Dash.Dash" (Transformation|GetActorLocation) "0, 0, 0" 0.5 1.0 0.0 0 0)
    (Character|LaunchCharacter (* (Math|Vector|GetForwardVector (Variables|Default|GetSprite)) 4e+02) false false)))

(fn ConstructionScript)

(fn Hit
  (for (_array_element _array_index) (Class|PanelWidget|GetAllChildren (Variables|/Game/Assets/WBP_HealthBar.WBP_HealthBar_C|GetHorizontalBox_40 (Variables|/Game/Character/BP_MyOwnHUD.BP_MyOwnHUD_C|GetWBP_HealthBar (Variables|Default|GetAs%20BP%20My%20Own%20HUD))))
    _)
  (Utilities|IsValid _array_element
    (:Is%20Valid
      (Widget|RemovefromParent _array_element)
      (if (== _array_index 0)
        (bind _returnvalue (Sprite|SetFlipbook (Variables|Default|GetSprite) "/Game/Character/FlipBooks_Cyber/FB_Death.FB_Death"))
        (if _returnvalue
          (Input|DisableInput 0)
          (Utilities|Time|SetTimerbyEvent (EventDispatchers|CreateEvent :!event Death) 0.7 true))))))

(fn Attack
  (for _array_element (Collision|GetOverlappingActors (Variables|Default|GetHitBox) "/Script/Paper2D.PaperCharacter" :!class /Script/Engine.PrimitiveComponent)
    (Game|Damage|ApplyDamage _array_element 0.4 0 0)))

(fn Death
  (Game|OpenLevel(byObjectReference) "/Game/MainMenuSystem/Levels/DeathScrren.DeathScrren"))